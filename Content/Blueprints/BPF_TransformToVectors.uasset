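; Blueprint function that splits a Transform into four vectors: TransformX, TransformY, TransformZ and TransformW.
; It converts the Transform to a matrix and copies the XYZ components of each plane, dropping each plane's W component.
; The X, Y and Z outputs carry the basis axes, and the W output carries the translation.
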(fn TransformtoVectors
  (params (Transform :type Transform))
  (bind _returnvalue (Math|Transform|ToMatrix(Transform) Transform))
  (bind (_xplane _yplane _zplane _wplane) (Utilities|Struct|BreakMatrix _returnvalue))
  (bind (_w _x _y _z) (Utilities|Struct|BreakPlane _wplane))
  (bind (_w_2 _x_2 _y_2 _z_2) (Utilities|Struct|BreakPlane _xplane))
  (bind (_w_3 _x_3 _y_3 _z_3) (Utilities|Struct|BreakPlane _yplane))
  (bind (_w_4 _x_4 _y_4 _z_4) (Utilities|Struct|BreakPlane _zplane))
  (return (Math|Vector|MakeVector _x_2 _y_2 _z_2) (Math|Vector|MakeVector _x_3 _y_3 _z_3) (Math|Vector|MakeVector _x_4 _y_4 _z_4) (Math|Vector|MakeVector _x _y _z)))
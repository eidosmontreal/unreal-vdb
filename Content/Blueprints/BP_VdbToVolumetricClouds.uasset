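; Actor that renders VDB volumes or volume textures as volumetric clouds by feeding them into a dynamic cloud material.
; Construction forces an identity transform and assigns the material instance to the VolumetricCloud; UpdateClouds also runs every Tick.
; For each cloud, up to MAXCLOUDS, it sets name-indexed parameters for inverse transform, 3D texture and volume bounds.
; A VdbToVolume actor's render target takes priority, with a static volume texture as fallback.
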(event EventBeginPlay)

(event Collision|EventActorBeginOverlap
  (params (OtherActor :type Actor%20Object%20Reference)))

(event EventTick
  (params (DeltaSeconds :type Float%20%28single-precision%29))
  (CallFunction|UpdateClouds))

(fn ConstructionScript
  (bind _cloud_mid (Variables|Default|GetCloud%20MID))
  (bind _cloud_material (Variables|Default|GetCloud%20Material))
  ;[1 1 1] Force Identity Transform
  (Transformation|SetActorTransform (Math|Transform|MakeTransform "0, 0, 0"))
  ;[1 1 1] Create Material Dynamic Instance
  (Utilities|IsValid _cloud_material
    (:Is%20Valid
      (CallFunction|CreateandAssignMID _cloud_mid _cloud_material)
      (Rendering|Material|SetMaterial (Variables|Default|GetVolumetricCloud) _cloud_mid)
      (CallFunction|UpdateClouds))))

(fn AppendName
  (params (Variable :type String) (Param :type String))
  (return (Utilities|String|StringToName (Utilities|String|Append Variable " " Param))))

(fn UpdateClouds
  (bind _cloud_mid (Variables|Default|GetCloud%20MID))
  (bind _cloud_mid_2 (Variables|Default|GetCloud%20MID))
  (bind _clouds__max_3_ (Variables|Default|GetClouds%20%28Max%203%29))
  (bind _cloud_mid_3 (Variables|Default|GetCloud%20MID))
  (bind _cloud_mid_4 (Variables|Default|GetCloud%20MID))
  (bind _cloud_mid_5 (Variables|Default|GetCloud%20MID)
    (:then
      ;[1 1 1] Set Number of Clouds
      (Rendering|Material|SetScalarParameterValue _cloud_mid_5 "NbClouds" (Math|Conversions|ToFloat(Integer) (Math|Integer|Min(Integer) (Utilities|Array|Length _clouds__max_3_) (Variables|Default|GetMAX_CLOUDS))) :!class /Script/Engine.MaterialInstanceDynamic)
      ;[1 1 1] Loop through clouds
      (for (_array_element _array_index) _clouds__max_3_
        (LocalVariables|SetCurrent%20Cloud _array_element)
        (if (< _array_index (Variables|Default|GetMAX_CLOUDS))
          (LocalVariables|SetCloud%20Name (Utilities|String|Append (Utilities|String|MakeLiteralString "Cloud ") (Utilities|String|ToString(Integer) (+ _array_index 1))))
          ;[1 1 1] Cloud1 Transform
          (bind (_transformx _transformy _transformz _transformw) (CallFunction|TransformtoVectors (Math|Transform|InvertTransform (.Transform (Utilities|Struct|BreakS_VdbCloud (LocalVariables|GetCurrent%20Cloud))))))
          (bind _name (CallFunction|AppendName (LocalVariables|GetCloud%20Name) "Transform X"))
          (Class|MaterialInstanceDynamic|SetDoubleVectorParameterValue _cloud_mid_3 _name _transformx)
          (bind _name_2 (CallFunction|AppendName (LocalVariables|GetCloud%20Name) "Transform Y"))
          (Class|MaterialInstanceDynamic|SetDoubleVectorParameterValue _cloud_mid_3 _name_2 _transformy)
          (bind _name_3 (CallFunction|AppendName (LocalVariables|GetCloud%20Name) "Transform Z"))
          (Class|MaterialInstanceDynamic|SetDoubleVectorParameterValue _cloud_mid_3 _name_3 _transformz)
          (bind _name_4 (CallFunction|AppendName (LocalVariables|GetCloud%20Name) "Transform W"))
          (Class|MaterialInstanceDynamic|SetDoubleVectorParameterValue _cloud_mid_3 _name_4 _transformw)
          ;[1 1 1] Cloud1 Volume Texture
          (Utilities|IsValid (.VdbToVolumeActor (Utilities|Struct|BreakS_VdbCloud (LocalVariables|GetCurrent%20Cloud)))
            (:Is%20Valid
              (Utilities|IsValid (Variables|/Script/VolumeRuntime.VdbToVolumeTextureComponent|GetVolumeRenderTarget (Variables|/Script/VolumeRuntime.VdbToVolumeTextureActor|GetVdbToTexComponent (.VdbToVolumeActor (Utilities|Struct|BreakS_VdbCloud (LocalVariables|GetCurrent%20Cloud)))))
                (:Is%20Valid
                  (bind _name_5 (CallFunction|AppendName (LocalVariables|GetCloud%20Name) "3D Texture"))
                  (Rendering|Material|SetTextureParameterValue _cloud_mid_4 _name_5 (Variables|/Script/VolumeRuntime.VdbToVolumeTextureComponent|GetVolumeRenderTarget (Variables|/Script/VolumeRuntime.VdbToVolumeTextureActor|GetVdbToTexComponent (.VdbToVolumeActor (Utilities|Struct|BreakS_VdbCloud (LocalVariables|GetCurrent%20Cloud))))))
                  ;[1 1 1] Update Volume Scale/Offset/Uv
                  (bind _name_6 (CallFunction|AppendName (LocalVariables|GetCloud%20Name) "VolumeSize"))
                  (Class|MaterialInstanceDynamic|SetDoubleVectorParameterValue _cloud_mid_2 _name_6 (Class|VdbAssetComponent|GetVolumeSize (Variables|/Script/VolumeRuntime.VdbToVolumeTextureActor|GetAssetComponent (.VdbToVolumeActor (Utilities|Struct|BreakS_VdbCloud (LocalVariables|GetCurrent%20Cloud))))))
                  (bind _name_7 (CallFunction|AppendName (LocalVariables|GetCloud%20Name) "VolumeOffset"))
                  (Class|MaterialInstanceDynamic|SetDoubleVectorParameterValue _cloud_mid_2 _name_7 (Class|VdbAssetComponent|GetVolumeOffset (Variables|/Script/VolumeRuntime.VdbToVolumeTextureActor|GetAssetComponent (.VdbToVolumeActor (Utilities|Struct|BreakS_VdbCloud (LocalVariables|GetCurrent%20Cloud))))))
                  (bind _name_8 (CallFunction|AppendName (LocalVariables|GetCloud%20Name) "VolumeUvScale"))
                  (Class|MaterialInstanceDynamic|SetDoubleVectorParameterValue _cloud_mid_2 _name_8 (Class|VdbAssetComponent|GetVolumeUvScale (Variables|/Script/VolumeRuntime.VdbToVolumeTextureActor|GetAssetComponent (.VdbToVolumeActor (Utilities|Struct|BreakS_VdbCloud (LocalVariables|GetCurrent%20Cloud)))))))
                (:Is%20Not%20Valid
                  (Utilities|IsValid (.VolumeTexture (Utilities|Struct|BreakS_VdbCloud (LocalVariables|GetCurrent%20Cloud))) :!label _label
                    (:Is%20Valid
                      (bind _name_9 (CallFunction|AppendName (LocalVariables|GetCloud%20Name) "3D Texture"))
                      (Rendering|Material|SetTextureParameterValue _cloud_mid_4 _name_9 (.VolumeTexture (Utilities|Struct|BreakS_VdbCloud (LocalVariables|GetCurrent%20Cloud))))
                      ;[1 1 1] Set default values. We only need Volume Texture Size, but it`s not available in blueprint. Will have to do it in the material/shader instead
                      (bind _name_10 (CallFunction|AppendName (LocalVariables|GetCloud%20Name) "VolumeSize"))
                      (Class|MaterialInstanceDynamic|SetDoubleVectorParameterValue _cloud_mid _name_10 "0, 0, 0")
                      (bind _name_11 (CallFunction|AppendName (LocalVariables|GetCloud%20Name) "VolumeOffset"))
                      (Class|MaterialInstanceDynamic|SetDoubleVectorParameterValue _cloud_mid _name_11 "0, 0, 0")
                      (bind _name_12 (CallFunction|AppendName (LocalVariables|GetCloud%20Name) "VolumeUvScale"))
                      (Class|MaterialInstanceDynamic|SetDoubleVectorParameterValue _cloud_mid _name_12 "1.000000,1.000000,1.000000"))))))
            (:Is%20Not%20Valid
              (goto _label))))))
    (:else)))
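; Actor that displays a VDB volume as a dynamic mesh box driven by a volume-texture material.
; Rebuilds the box each tick and at construction from the asset component's volume size and offset.
; A dynamic material instance receives the UV scale and, when valid, the VdbToTex component's volume render target.
; Construction creates that instance only when a parent material is set.
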(event EventBeginPlay)

(event Collision|EventActorBeginOverlap
  (params (OtherActor :type Actor%20Object%20Reference)))

(event EventTick
  (params (DeltaSeconds :type Float%20%28single-precision%29))
  (CallFunction|UpdateMesh)
  (CallFunction|UpdateMaterial))

(event EventUpdateDynamicMesh)

(fn ConstructionScript
  (bind _mid (Variables|MasterMaterial|GetMID))
  ;[1 1 1] Create Material Dynamic Instance
  (bind _material (Variables|MasterMaterial|GetMaterial)
    (:then
      (CallFunction|CreateandAssignMID _mid _material)
      (Rendering|Material|SetMaterial (Variables|Default|GetDynamicMeshComponent) 0 _mid)
      (CallFunction|UpdateMesh)
      (CallFunction|UpdateMaterial))
    (:else)))

(fn UpdateMesh
  (bind _assetcomponent (Variables|Default|GetAssetComponent))
  (bind _returnvalue (Class|VdbAssetComponent|GetVolumeSize _assetcomponent))
  (bind _returnvalue_2 (Class|VdbAssetComponent|GetVolumeOffset _assetcomponent))
  (bind _returnvalue_3 (DynamicMeshComponent|GetDynamicMesh (Variables|Default|GetDynamicMeshComponent)))
  (bind _returnvalue_4 (DynamicMesh|Reset _returnvalue_3))
  (Class|GeometryScriptLibraryMeshPrimitiveFunctions|AppendBox :TargetMesh _returnvalue_4 :Transform (Math|Transform|MakeTransform (Math|Vector|MakeVector (+ (.x _returnvalue_2) (* (.x _returnvalue) 0.5)) (+ (.y _returnvalue_2) (* (.y _returnvalue) 0.5)) (+ (.z _returnvalue_2) (* (.z _returnvalue) 0.5))) "0, 0, 0" "1.000000,1.000000,1.000000") :DimensionX (.x _returnvalue) :DimensionY (.y _returnvalue) :DimensionZ (.z _returnvalue) :Origin "Center" :Debug 0))

(fn UpdateMaterial
  (bind _mid (Variables|MasterMaterial|GetMID)
    (:then
      (Class|MaterialInstanceDynamic|SetDoubleVectorParameterValue _mid "UvScale" (Class|VdbAssetComponent|GetVolumeUvScale (Variables|Default|GetAssetComponent)))
      (bind _volumerendertarget (Variables|/Script/VolumeRuntime.VdbToVolumeTextureComponent|GetVolumeRenderTarget (Variables|Default|GetVdbToTexComponent))
        (:then
          (Rendering|Material|SetTextureParameterValue _mid "VolumeTexture" _volumerendertarget))
        (:else)))
    (:else)))